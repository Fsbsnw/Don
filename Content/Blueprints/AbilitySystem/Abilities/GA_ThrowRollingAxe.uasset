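; GA_ThrowRollingAxe is a gameplay ability for a ranged axe attack aimed at the mouse cursor.
; On activation it commits its cooldown and snaps the avatar's yaw toward a cursor trace hit from player controller 0.
; It plays the axe range-attack montage and calls CauseDamage as the montage starts, without waiting for a notify.
; The ability ends when the montage completes, blends out or is interrupted or cancelled.
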(event Ability|EventActivateAbility
  (Ability|CommitAbilityCooldown false)
  (CallFunction|RotatetoCursor)
  (|PlayMontageandWaitProxy "None" "/Game/Blueprints/Character/Player/Montage/AM_Axe_RangeAttack.AM_Axe_RangeAttack" 1.0 "None" true 1.0 0.0
    (:then
      (Class|DonDamageGameplayAbility|CauseDamage))
    (:OnCompleted
      (Ability|EndAbility :!label _label))
    (:OnBlendOut
      (goto _label))
    (:OnInterrupted
      (goto _label))
    (:OnCancelled
      (goto _label))))

(fn RotatetoCursor
  (Transformation|SetActorRotation (Ability|GetAvatarActorfromActorInfo) (Math|Rotator|MakeRotator 0.0 0.0 (.yaw (Math|Rotator|FindLookatRotation (Transformation|GetActorLocation (Ability|GetAvatarActorfromActorInfo)) (.ImpactPoint (Collision|BreakHitResult (.HitResult (Game|Player|GetHitResultUnderCursorbyChannel (Game|GetPlayerController 0) "TraceTypeQuery1" true)))))))))