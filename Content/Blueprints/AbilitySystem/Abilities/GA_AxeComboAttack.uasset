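; Gameplay ability for a three-step axe combo melee attack that turns the avatar toward the cursor before each swing.
; Each swing plays a montage section, and its FireBolt event triggers a sphere overlap in front of the avatar that damages enemy pawns.
; Montage events toggle a loose window-open tag; input during that window advances the combo.
; The interrupt handler avoids ending the ability when a chained swing replaces the previous one.
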(event Ability|EventActivateAbility
  (Ability|CommitAbility)
  (CallFunction|RotatetoCursor :!label _label)
  (|PlayMontageandWaitProxy "None" "/Game/Blueprints/Character/Player/Montage/AM_ComboAttack.AM_ComboAttack" 1.0 (Utilities|Array|Get(acopy) (Variables|Default|GetComboSections) (Variables|Default|GetCachedComboIndex)) false 1.0 0.0
    (:then
      (Variables|Default|SetComboIndex (Variables|Default|GetCachedComboIndex))
      (Ability|Tasks|WaitGameplayEvent "(TagName=\"Event.Montage.FireBolt\")" 0 true
        (:then
          (bind _payload (Ability|Tasks|WaitGameplayEvent "(TagName=\"Event.Montage.ComboAttack\")" 0 false false)
            (:then
              (Ability|Tasks|WaitInputPress false :!label _label_2
                (:OnPress
                  (if (GameplayTags|HasMatchingGameplayTag (Ability|GetAbilitySystemComponentfromActorInfo) "(TagName=\"Event.Montage.ComboAttack.WindowOpen\")")
                    (CallFunction|RemoveAbilityTag)
                    (bind _result (Math|Integer|IncrementInt (Variables|Default|GetCachedComboIndex))
                      (:%20%20
                        (if (not (>= _result 3))
                          (goto _label))))
                    (else
                      (goto _label_2))))))
            (:EventReceived
              (if (== (.EventTag (Utilities|Struct|BreakGameplayEventData _payload)) "(TagName=\"Event.Montage.ComboAttack.WindowOpen\")")
                (CallFunction|AddAbilityTag)
                (else
                  (CallFunction|RemoveAbilityTag))))))
        (:EventReceived
          (bind _outactors (Collision|SphereOverlapActors (CallFunction|GetCombatCenter) (Variables|Default|GetCombatRadius) (Variables|Default|GetObject%20Types) "/Script/Don.DonEnemyPawn" (Variables|Default|GetActors%20to%20Ignore)))
          (for _array_element _outactors
            (Audio|PlaySoundatLocation "/Game/Blueprints/Sounds/axe-hit-flesh.axe-hit-flesh" (Transformation|GetActorLocation _array_element) "0, 0, 0" 2.0 1.0 0.0 0 0 0 0)
            (Class|DonDamageGameplayAbility|CauseDamage _array_element)
            (Utilities|Array|AddUnique (Variables|Default|GetActors%20to%20Ignore) _array_element))
          (Utilities|Array|Clear (Variables|Default|GetActors%20to%20Ignore)))))
    (:OnCompleted
      (Ability|EndAbility :!label _label_3))
    (:OnBlendOut
      (goto _label_3))
    (:OnInterrupted
      (if (>= (Variables|Default|GetComboIndex) 2)
        (goto _label_3)
        (elif (== (Variables|Default|GetComboIndex) (Variables|Default|GetCachedComboIndex))
          (goto _label_3))))
    (:OnCancelled
      (goto _label_3))))

(event Ability|EventOnEndAbility
  (params (bWasCancelled :type Boolean))
  (CallFunction|RemoveAbilityTag))

(fn RemoveAbilityTag
  (Ability|GameplayEffect|RemoveLooseGameplayTags (Ability|GetAvatarActorfromActorInfo) (GameplayTags|MakeLiteralGameplayTagContainer "(GameplayTags=((TagName=\"Event.Montage.ComboAttack.WindowOpen\")))")))

(fn AddAbilityTag
  (Ability|GameplayEffect|AddLooseGameplayTags (Ability|GetAvatarActorfromActorInfo) (GameplayTags|MakeLiteralGameplayTagContainer "(GameplayTags=((TagName=\"Event.Montage.ComboAttack.WindowOpen\")))")))

(fn RotatetoCursor
  (Transformation|SetActorRotation (Ability|GetAvatarActorfromActorInfo) (Math|Rotator|MakeRotator 0.0 0.0 (.yaw (Math|Rotator|FindLookatRotation (Transformation|GetActorLocation (Ability|GetAvatarActorfromActorInfo)) (.ImpactPoint (Collision|BreakHitResult (.HitResult (Game|Player|GetHitResultUnderCursorbyChannel (Game|GetPlayerController 0) "TraceTypeQuery1" true)))))))))

(fn GetCombatCenter
  (bind _returnvalue (Ability|GetAvatarActorfromActorInfo))
  (return (+ (* (Transformation|GetActorForwardVector _returnvalue) 1e+02) (Transformation|GetActorLocation _returnvalue))))