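; Gameplay ability for an axe slash that turns the avatar to face the cursor and damages nearby enemies.
; On activation it commits the cooldown, snaps yaw toward the cursor hit point, and plays the slash montage.
; The montage's Event.Montage.FireBolt gameplay event triggers a sphere overlap around the avatar, damaging every DonEnemy found, with no arc filtering.
; The ability ends when the montage completes, blends out, or is interrupted or cancelled.
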(event Ability|EventActivateAbility
  (Ability|CommitAbilityCooldown false)
  (CallFunction|RotatetoCursor)
  (|PlayMontageandWaitProxy "None" "/Game/Blueprints/Character/Player/Montage/AM_Axe_Slash.AM_Axe_Slash" 1.0 "None" true 1.0 0.0
    (:then
      (Ability|Tasks|WaitGameplayEvent "(TagName=\"Event.Montage.FireBolt\")" 0 true
        (:EventReceived
          (bind _outactors (Collision|SphereOverlapActors (Transformation|GetActorLocation (Ability|GetAvatarActorfromActorInfo)) (Variables|Default|GetAttackRadius) (Variables|Default|GetObject%20Types) "/Script/Don.DonEnemy"))
          (for _array_element _outactors
            (Class|DonDamageGameplayAbility|CauseDamage _array_element)))))
    (:OnCompleted
      (Ability|EndAbility :!label _label))
    (:OnBlendOut
      (goto _label))
    (:OnInterrupted
      (goto _label))
    (:OnCancelled
      (goto _label))))

(fn RotatetoCursor
  (Transformation|SetActorRotation (Ability|GetAvatarActorfromActorInfo) (Math|Rotator|MakeRotator 0.0 0.0 (.yaw (Math|Rotator|FindLookatRotation (Transformation|GetActorLocation (Ability|GetAvatarActorfromActorInfo)) (.ImpactPoint (Collision|BreakHitResult (.HitResult (Game|Player|GetHitResultUnderCursorbyChannel (Game|GetPlayerController 0) "TraceTypeQuery1" true)))))))))