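; Gameplay ability for a teleport slash attack that runs only when a combat target is found.
; Activation commits cooldown, attaches a skeletal trail effect and disables character movement.
; TeleporttoTarget plays the slash montage, waits for a gameplay event, then damages enemies in a sphere around the avatar, with a gameplay cue and brief global time-dilation hit-stop.
; RequestEndAbility removes the trail, restores walking and ends the ability.
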(event Ability|EventActivateAbility
  ;[1 1 1] Activate Ability
  (bind _returnvalue (Class|TeleportAttack|FindCombatTarget))
  (if _returnvalue
    (Ability|CommitAbilityCooldown false)
    (bind _asdon_character_base (Utilities|Casting|CastToDonCharacterBase (Ability|GetAvatarActorfromActorInfo)))
    (bind _returnvalue_2 (Niagara|SpawnSystemAttached "/Game/Blueprints/AbilitySystem/Abilities/Niagara/NS_SkeletalTrail.NS_SkeletalTrail" (Variables|/Script/Engine.Character|GetMesh _asdon_character_base) "" "0, 0, 0" "0, 0, 0" "SnapToTargetIncludingScale" false))
    (Variables|Default|SetNSTrail _returnvalue_2)
    (bind _ascharacter (Utilities|Casting|CastToCharacter (Ability|GetAvatarActorfromActorInfo)))
    (Pawn|Components|CharacterMovement|SetMovementMode (Variables|/Script/Engine.Character|GetCharacterMovement _ascharacter) "MOVE_None" 0)
    (else
      (Ability|EndAbility))))

(event EventTeleporttoTarget
  ;[1 1 1] Visual Effect
  (|PlayMontageandWaitProxy "None" "/Game/Blueprints/Character/Player/Montage/AM_TeleportSlash.AM_TeleportSlash" 0.75 "None" true 1.0 0.0
    (:then
      (Ability|Tasks|WaitGameplayEvent "(TagName=\"Event.Montage.FireBolt\")" 0 true
        (:EventReceived
          (bind (_outactors _returnvalue) (Collision|SphereOverlapActors (Transformation|GetActorLocation (Ability|GetAvatarActorfromActorInfo)) (Variables|Default|GetAttackRange) (Variables|Default|GetObject%20Types) "/Script/Don.DonEnemy"))
          (if _returnvalue
            (for _array_element _outactors
              (Class|DonDamageGameplayAbility|CauseDamage _array_element)
              (GameplayCue|ExecuteGameplayCue :GameplayCueTag "(TagName=\"GameplayCue\")")
              (Utilities|Time|SetGlobalTimeDilation 0.05)
              (Utilities|FlowControl|Delay (Class|TeleportAttack|GetDelayMultiplier))
              (Utilities|Time|SetGlobalTimeDilation 1.0))))))))

(event EventRequestEndAbility
  ;[1 1 1] End Ability
  (Components|DestroyComponent (Variables|Default|GetNSTrail))
  (bind _ascharacter (Utilities|Casting|CastToCharacter (Ability|GetAvatarActorfromActorInfo)))
  (Pawn|Components|CharacterMovement|SetMovementMode (Variables|/Script/Engine.Character|GetCharacterMovement _ascharacter) "MOVE_Walking" 0)
  (Ability|EndAbility))