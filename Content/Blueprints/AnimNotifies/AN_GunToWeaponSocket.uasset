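; Anim notify that moves the player's weapon between sockets on the animated mesh during an animation.
; It casts the mesh owner to BP_Player_1 and gets the player weapon, doing nothing for other owners.
; It snaps the weapon's root to the Weapon_rHand socket, or to ik_hand_gun when the Reverse flag is set.
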(fn ReceivedNotify
  (params (MeshComp :type Skeletal%20Mesh%20Component%20Object%20Reference) (Animation :type Anim%20Sequence%20Base%20Object%20Reference) (EventReference :type Anim%20Notify%20Event%20Reference%20Structure%20%28by%20ref%29))
  (bind _output_get (LocalVariables|SetMesh MeshComp))
  (bind _asbp_player_1 (Utilities|Casting|CastToBP_Player_1 (Components|GetOwner _output_get)))
  (bind _returnvalue (Class|DonCharacter|GetPlayerWeapon _asbp_player_1))
  (if (Variables|Default|GetbReverse)
    (Transformation|AttachComponentToComponent (Variables|/Script/Engine.Actor|GetRootComponent _returnvalue) (LocalVariables|GetMesh) "ik_hand_gun" "SnapToTarget" "SnapToTarget" "SnapToTarget" true)
    (else
      (Transformation|AttachComponentToComponent (Variables|/Script/Engine.Actor|GetRootComponent _returnvalue) (LocalVariables|GetMesh) "Weapon_rHand" "SnapToTarget" "SnapToTarget" "SnapToTarget" true)))
  (return false))