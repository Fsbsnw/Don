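; AN_MontageEvent is an anim notify that sends a gameplay event with its EventTag to the mesh's owning actor.
; It also spawns a Niagara trail attached to the mesh at ik_hand_gun, setting its thickness and its lifetime from the Lifetime variable.
; An alternate, thicker trail setup using a different Niagara system is present but unconnected, so it never runs.
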(fn ReceivedNotify
  (params (MeshComp :type Skeletal%20Mesh%20Component%20Object%20Reference) (Animation :type Anim%20Sequence%20Base%20Object%20Reference) (EventReference :type Anim%20Notify%20Event%20Reference%20Structure%20%28by%20ref%29))
  (bind _output_get (LocalVariables|SetOwner (Components|GetOwner MeshComp)))
  (Ability|SendGameplayEventtoActor _output_get (Variables|Default|GetEventTag))
  (LocalVariables|SetThickness 75.0)
  (LocalVariables|SetNiagaraTrail "/Game/SwordTrailVFX/VFX/NS_Trail_11.NS_Trail_11")
  (bind _returnvalue (Niagara|SpawnSystemAttached (LocalVariables|GetNiagaraTrail) MeshComp "ik_hand_gun" "0, 0, 0" "0, 0, 0" "KeepRelativeOffset" false))
  (Niagara|SetNiagaraVariable(Float) _returnvalue "user.Thickness" (LocalVariables|GetThickness))
  (Niagara|SetNiagaraVariable(Float) _returnvalue "user.Lifetime" (LocalVariables|GetLifetime))
  (return false))