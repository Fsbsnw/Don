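; Base enemy Blueprint that provides a physical hit reaction on the skeletal mesh.
; PhysicsHitReact skips sweeping attacks; otherwise it enables physics collision, simulates bodies from the hit bone down and applies a velocity-change impulse there.
; A BlendWeight timeline drives those bodies' physics blend weight, then returns the mesh to query-only collision when finished, without explicitly switching simulation off.
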(event Custom|PhysicsHitReact
  (params (HitBone :type Name) (bSweepingAttack :type Boolean))
  (if (not bSweepingAttack)
    (Collision|SetCollisionEnabled (Variables|Character|GetMesh) "QueryAndPhysics")
    (Class|SkeletalMeshComponent|SetAllBodiesBelowSimulatePhysics (Variables|Character|GetMesh) (Variables|Default|GetHit%20Bone) true true)
    (Utilities|FlowControl|Sequence
      (:then_0
        (bind _weight (Timeline|BlendWeight PlayFromStart)
          (:Update
            (Class|SkeletalMeshComponent|SetAllBodiesBelowPhysicsBlendWeight (Variables|Character|GetMesh) (Variables|Default|GetHit%20Bone) _weight false true))
          (:Finished
            (Collision|SetCollisionEnabled (Variables|Character|GetMesh) "QueryOnly"))))
      (:then_1
        (Physics|AddImpulse (Variables|Character|GetMesh) (Variables|Default|GetImpulse) (Variables|Default|GetHit%20Bone) true)))))

(fn ConstructionScript)